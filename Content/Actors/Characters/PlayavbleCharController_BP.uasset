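; Player controller that lets the player paint grass onto the ground with the mouse.
; While the Editor_Paint axis is at full value, it deprojects the cursor and runs a complex line trace into the world.
; On a Ground_BP hit, it converts the hit to a UV through FindCollisionUV and passes it to that actor's DrawBrush with the BasicGrass texture.
; An EditorHUD widget setup is present but never runs.
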(event EventBeginPlay
  (|CallParentFunction))

(event Input|AxisEvents|InputAxisEditor_Paint
  (params (AxisValue :type Float%20%28single-precision%29))
  (bind (_worldlocation _worlddirection) (Game|Player|ConvertMouseLocationToWorldSpace))
  (if (== AxisValue 1.0)
    (bind (_outhit _returnvalue) (Collision|LineTraceByChannel _worldlocation (+ _worldlocation (* _worlddirection 1e+04)) "TraceTypeQuery3" true 0 "None"))
    (if _returnvalue
      (bind _asground_bp (Utilities|Casting|CastToGround_BP (.HitActor (Collision|BreakHitResult _outhit))))
      (Default|DrawBrush _asground_bp "/Game/Materials/Textures/BasicGrass.BasicGrass" 5e+01 (.UV (Class|GameplayStatics|FindCollisionUV _outhit))))))

(fn ConstructionScript)