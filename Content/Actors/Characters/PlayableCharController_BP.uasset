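; Player controller that separates a free-moving camera from the playable character, which moves by mouse click on a tile grid.
; On BeginPlay it shows the cursor, spawns a CameraPawn at the controlled pawn and views through it, forwarding movement axes to that camera.
; Clicks trace under the cursor and instantly relocate the controlled pawn to the hit tile's center, using sign-aware modulo snapping on a 50-unit grid.
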(event EventBeginPlay
  (bind _returnvalue (Pawn|GetControlledPawn))
  (bind _returnvalue_2 (Transformation|GetActorTransform _returnvalue))
  (Variables|Default|SetbShowMouseCursor true)
  (bind _returnvalue_3 (Game|SpawnActorfromClass "/Game/Actors/Characters/CameraPawn.CameraPawn_C" (Math|Transform|MakeTransform (.location _returnvalue_2) (.rotation _returnvalue_2) "1,1,1") "Undefined" 0 0))
  (bind _output_get (Variables|Default|SetCameraPawn _returnvalue_3))
  (Game|Player|SetViewTargetwithBlend _output_get 0.0 "VTBlend_Linear" 0.0 false))

(event Input|ActionEvents|InputActionMouseClick
  (params (Key :type Key%20Structure))
  (:Pressed
    (CallFunction|MouseClickMovement)))

(event Input|AxisEvents|InputAxisMovement_Forward
  (params (AxisValue :type Float%20%28single-precision%29))
  (Default|Movement (Variables|Default|GetCameraPawn) (* "1.000000, 0, 0" AxisValue)))

(event Input|AxisEvents|InputAxisMovement_Right
  (params (AxisValue :type Float%20%28single-precision%29))
  (Default|Movement (Variables|Default|GetCameraPawn) (* "0.000000,1.000000, 0" AxisValue)))

(fn ConstructionScript)

(fn MouseClickMovement
  (bind (_worldlocation _worlddirection) (Game|Player|ConvertMouseLocationToWorldSpace))
  (bind (_outhit _returnvalue) (Collision|LineTraceByChannel _worldlocation (+ _worldlocation (* _worlddirection 1e+04)) "TraceTypeQuery3" false 0 "None"))
  (if _returnvalue
    (bind _tile_centre (CallFunction|LocateTilePos (.Location (Collision|BreakHitResult _outhit))))
    (Transformation|SetActorLocation (Pawn|GetControlledPawn) _tile_centre false false)))

(fn LocateTilePos
  (params (Click%20Pos :type Vector))
  (bind (_x _y) (Math|Vector|BreakVector Click%20Pos))
  (bind (_x_2 _y_2 _z) (Math|Vector|BreakVector Click%20Pos))
  (return (+ (Math|Vector|MakeVector (- _x_2 (Math|Float|%(Float) _x_2 5e+01)) (- _y_2 (Math|Float|%(Float) _y_2 5e+01)) _z) (Math|Vector|MakeVector (* (Math|Float|Sign(Float) _x) 25.0) (* (Math|Float|Sign(Float) _y) 25.0) 0.0))))