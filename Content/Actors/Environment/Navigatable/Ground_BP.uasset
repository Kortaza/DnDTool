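; Navigatable ground actor Blueprint with a prototype for painting brush textures onto a render target.
; DrawBrush sets the texture on a brush material instance and draws it to the target via canvas, centered on a normalized location.
; The setup that creates the render target, shows it on GroundPlane and creates the brush material is disconnected from BeginPlay, so it never runs.
; The construction script is also empty, leaving its GroundMaterial instance node unused.
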(event EventBeginPlay)

(fn ConstructionScript)

(fn DrawBrush
  (params (BrushTexture :type Texture%202D%20Object%20Reference) (BrushSize :type Float%20%28single-precision%29) (DrawLocation :type Vector%202D%20Structure))
  (Utilities|FlowControl|Sequence
    (:then_0
      (Rendering|Material|SetTextureParameterValue (Variables|Default|GetBrushMaterial%20test) "BrushTexture" BrushTexture))
    (:then_1
      (bind (_canvas _size _context) (Rendering|BeginDrawCanvastoRenderTarget (Variables|Default|GetRenderTarget%20test)))
      (Canvas|DrawMaterial :self _canvas :RenderMaterial (Variables|Default|GetBrushMaterial%20test) :ScreenPosition (- (* _size DrawLocation) (/ BrushSize 2.0)) :ScreenSize (Math|Vector2D|MakeVector2D BrushSize BrushSize) :Rotation 9e+01)
      (Rendering|EndDrawCanvastoRenderTarget _context))))